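; BP_AIUnit is a clickable unit that lives on the BP_Grid tile map and moves along tile paths.
; On BeginPlay it finds the grid, stores the closest tile as its GridIndex and snaps to it.
; Clicking its Cone reports it to BP_PlayerController as the newly selected unit.
; For movement, it rebuilds the grid's shared spline from path tiles, raised by capsule half-height, and a timeline drives its location and rotation along it.
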(event OnClicked(Cone)
  (params (TouchedComponent :type Primitive%20Component%20Object%20Reference) (ButtonPressed :type Key%20Structure :default "None"))
  (if (!= (Variables|/Game/BP_PlayerController.BP_PlayerController_C|GetSelectedUnit (Variables|Default|Getplayercontroller)) self)
    (Default|EventNewUnitSelected (Variables|Default|Getplayercontroller) self)))

(event Custom|Event_MoveAlongThePath
  (params (Path :type Array%20of%20Vector%202D%20Structures))
  (bind _grid (Variables|Default|Getgrid))
  (bind _spline (Variables|/Game/BP_Grid.BP_Grid_C|GetSpline _grid))
  (Variables|Default|SetPath Path)
  (Spline|ClearSplinePoints (Variables|/Game/BP_Grid.BP_Grid_C|GetSpline (Variables|Default|Getgrid)) true)
  (for _array_element (Variables|Default|GetPath)
    (Spline|AddSplinePoint (Variables|/Game/BP_Grid.BP_Grid_C|GetSpline (Variables|Default|Getgrid)) (Math|Vector|MakeVector (.x (.worldlocation (.Value (Utilities|Map|Find (Variables|/Game/BP_Grid.BP_Grid_C|Getstruct_Tiles (Variables|Default|Getgrid)) _array_element)))) (.y (.worldlocation (.Value (Utilities|Map|Find (Variables|/Game/BP_Grid.BP_Grid_C|Getstruct_Tiles (Variables|Default|Getgrid)) _array_element)))) (+ (.z (.worldlocation (.Value (Utilities|Map|Find (Variables|/Game/BP_Grid.BP_Grid_C|Getstruct_Tiles (Variables|Default|Getgrid)) _array_element)))) (Variables|/Script/Engine.CapsuleComponent|GetCapsuleHalfHeight (Variables|Collision|GetCapsuleComponent)))) "World" true))
  (bind _progression (Timeline|MoveAlongthePathTimeLine PlayFromStart)
    (:Update
      (Transformation|SetActorTransform self (Math|Transform|MakeTransform (Spline|GetLocationatDistanceAlongSpline _spline (* _progression (Spline|GetSplineLength _spline)) "World") (Spline|GetRotationatDistanceAlongSpline _spline (* _progression (Spline|GetSplineLength _spline)) "World") "1,1,1")))))

(event EventBeginPlay
  (Variables|Default|Setplayercontroller (.AsBP%20Player%20Controller (Utilities|Casting|CastToBP_PlayerController (Game|GetPlayerController 0))))
  (bind _outactors (Actor|GetAllActorsOfClass "/Game/BP_Grid.BP_Grid_C"))
  (Variables|Default|Setgrid (Utilities|Array|Get(acopy) _outactors))
  (CallFunction|SetGridIndexandSnaptoLocation))

(event Collision|EventActorBeginOverlap
  (params (OtherActor :type Actor%20Object%20Reference)))

(event EventTick
  (params (DeltaSeconds :type Float%20%28single-precision%29)))

(fn ConstructionScript)

(fn SetGridIndexandSnaptoLocation
  (LocalVariables|SetclosestDistance 1e+08)
  (bind _keys (Utilities|Map|Keys (Variables|/Game/BP_Grid.BP_Grid_C|Getstruct_Tiles (Variables|Default|Getgrid))))
  (for _array_element _keys
    (if (< (Math|Vector|VectorLength (- (.worldlocation (.Value (Utilities|Map|Find (Variables|/Game/BP_Grid.BP_Grid_C|Getstruct_Tiles (Variables|Default|Getgrid)) _array_element))) (Transformation|GetActorLocation self))) (LocalVariables|GetclosestDistance))
      (LocalVariables|SetclosestDistance (Math|Vector|VectorLength (- (.worldlocation (.Value (Utilities|Map|Find (Variables|/Game/BP_Grid.BP_Grid_C|Getstruct_Tiles (Variables|Default|Getgrid)) _array_element))) (Transformation|GetActorLocation self))))
      (LocalVariables|SetclosestIndex _array_element)))
  (Variables|Default|SetgridIndex (LocalVariables|GetclosestIndex))
  (Transformation|SetActorLocation (.worldlocation (.Value (Utilities|Map|Find (Variables|/Game/BP_Grid.BP_Grid_C|Getstruct_Tiles (Variables|Default|Getgrid)) (LocalVariables|GetclosestIndex)))) false false))