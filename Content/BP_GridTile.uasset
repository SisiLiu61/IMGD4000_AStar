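; BP_GridTile is a single clickable grid tile that shows its ground type and interaction state through color.
; After a short BeginPlay delay it colors itself, scales its cube flat to BPGrid's tile size, and passes grid and index to its W_GridTile widget.
; Hover and click events set state flags and notify BPGrid.
; SetTileColor reads BPGrid's tile data, layers selected, hovered and in-path overrides, then sets a material parameter.
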(event OnBeginCursorOver(Cube)
  (params (TouchedComponent :type Primitive%20Component%20Object%20Reference))
  (CallFunction|EventStartOverTile)
  (Default|EventNewTileOvered (Variables|Default|GetBP_Grid) self))

(event OnEndCursorOver(Cube)
  (params (TouchedComponent :type Primitive%20Component%20Object%20Reference)))

(event OnClicked(Cube)
  (params (TouchedComponent :type Primitive%20Component%20Object%20Reference) (ButtonPressed :type Key%20Structure :default "None"))
  (CallFunction|EventSelectTile)
  (Default|EventNewTileSelected (Variables|Default|GetBP_Grid) self))

(event Custom|Event_DeselectTile
  (Variables|Default|SetbIsSelected false)
  (CallFunction|SetTileColor))

(event Custom|Event_SelectTile
  (Variables|Default|SetbIsSelected true)
  (CallFunction|SetTileColor))

(event Custom|Event_EndOverTile
  (Variables|Default|SetbIsOvered false)
  (CallFunction|SetTileColor))

(event Custom|Event_StartOverTile
  (Variables|Default|SetbIsOvered true)
  (CallFunction|SetTileColor))

(event Custom|Event_isInPath
  (params (bIsinPath :type Boolean))
  (Variables|Default|SetisinPath bIsinPath)
  (CallFunction|SetTileColor))

(event EventBeginPlay
  (Utilities|FlowControl|Delay 0.2)
  (CallFunction|SetTileColor)
  (CallFunction|SetTileSize)
  (CallFunction|SetWidgetVariables))

(event Collision|EventActorBeginOverlap
  (params (OtherActor :type Actor%20Object%20Reference)))

(event EventTick
  (params (DeltaSeconds :type Float%20%28single-precision%29)))

(fn ConstructionScript)

(fn SetTileColor
  (Utilities|FlowControl|Sequence
    (:then_0
      (switch Utilities|FlowControl|Switch|SwitchonEnum_GroundTypes (.groundtype (CallFunction|GetTileData))
        (:NewEnumerator0
          (LocalVariables|SetTitleColor "(R=1.000000,G=0.887153,B=0.887153,A=1.000000)"))
        (:NewEnumerator1
          (LocalVariables|SetTitleColor "(R=0.427327,G=0.546875,B=0.198490,A=1.000000)"))
        (:NewEnumerator2
          (LocalVariables|SetTitleColor "(R=0.939236,G=0.807359,B=0.073378,A=1.000000)"))
        (:NewEnumerator3
          (LocalVariables|SetTitleColor "(R=0.845486,G=0.000000,B=0.037123,A=1.000000)"))
        (:NewEnumerator4
          (LocalVariables|SetTitleColor "(R=0.000000,G=0.000000,B=0.000000,A=1.000000)"))))
    (:then_1
      (if (Variables|Default|GetbIsSelected)
        (LocalVariables|SetTitleColor "(R=0.128965,G=0.100287,B=0.734375,A=1.000000)")))
    (:then_2
      (if (Variables|Default|GetbIsOvered)
        (LocalVariables|SetTitleColor "(R=0.128965,G=0.100287,B=0.734375,A=1.000000)")))
    (:then_3
      (if (Variables|Default|GetisinPath)
        (LocalVariables|SetTitleColor "(R=0.000159,G=0.001872,B=0.211805,A=1.000000)")))
    (:then_4
      (Rendering|Material|SetVectorParameterValueonMaterials (Variables|Default|GetCube) "Color" (Math|Conversions|ToVector(LinearColor) (LocalVariables|GetTitleColor))))))

(fn GetTileData
  (return (.Value (Utilities|Map|Find (Variables|/Game/BP_Grid.BP_Grid_C|Getstruct_Tiles (Variables|Default|GetBP_Grid)) (Variables|Default|GetgridIndex)))))

(fn SetTileSize
  (bind _bp_grid (Variables|Default|GetBP_Grid))
  (bind _cube (Variables|Default|GetCube))
  (bind _returnvalue (Transformation|GetWorldScale _cube))
  (bind _tilesize (Variables|/Game/BP_Grid.BP_Grid_C|GetTileSize _bp_grid))
  (bind _returnvalue_2 (/ _tilesize 5e+01))
  (bind _returnvalue_3 (* _returnvalue _returnvalue_2))
  (Transformation|SetWorldScale3D (Variables|Default|GetCube) (Math|Vector|MakeVector (.x _returnvalue_3) (.y _returnvalue_3) 0.0)))

(fn SetWidgetVariables
  (bind _asw_grid_tile (Utilities|Casting|CastToW_GridTile (UserInterface|GetUserWidgetObject (Variables|Default|GetWidget))))
  (Variables|/Game/W_GridTile.W_GridTile_C|Setgrid _asw_grid_tile (Variables|Default|GetBP_Grid))
  (Variables|/Game/W_GridTile.W_GridTile_C|SetgridIndex _asw_grid_tile (Variables|Default|GetgridIndex)))