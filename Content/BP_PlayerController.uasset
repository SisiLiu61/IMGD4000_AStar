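; Player controller that holds a selected AI unit and relays movement paths to it.
; A selection event stores the incoming unit only when no valid unit is already selected.
; A new-path event passes the path to the selected unit's move-along-path event if that unit is valid.
; The R key gathers all BP_Base_Obstacle actors and loops over them with an empty body.
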(event Custom|Event_NewUnitSelected
  (params (AIUnit :type BP%20AI%20Unit%20Object%20Reference))
  (Utilities|IsValid (Variables|Default|GetSelectedUnit)
    (:Is%20Not%20Valid
      (Variables|Default|SetSelectedUnit AIUnit))))

(event Custom|Event_NewPathAvailable
  (params (Path :type Array%20of%20Vector%202D%20Structures))
  (Utilities|IsValid (Variables|Default|GetSelectedUnit)
    (:Is%20Valid
      (Default|EventMoveAlongthePath (Variables|Default|GetSelectedUnit) Path))))

(event EventBeginPlay)

(event EventTick
  (params (DeltaSeconds :type Float%20%28single-precision%29)))

(event Input|KeyboardEvents|R
  (params (Key :type Key%20Structure :default "None"))
  (:Pressed
    (bind _outactors (Actor|GetAllActorsOfClass "/Game/BP_Base_Obstacle.BP_Base_Obstacle_C"))
    (for _array_element _outactors
      _)))

(fn ConstructionScript)