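; BP_Grid is a tile grid actor that provides terrain-weighted pathfinding between a selected and a hovered tile.
; Sphere traces classify each cell's ground type and cost into a tile map, previewed with debug shapes in the Construction Script.
; At BeginPlay it spawns BP_GridTile actors from that map.
; Hovering runs four-way A* with a Manhattan heuristic and highlights the path; selecting a tile sends the path to BP_PlayerController.
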(event Custom|Event_NewTileSelected
  (params (selectedTile :type BP%20Grid%20Tile%20Object%20Reference))
  (Utilities|IsValid (Variables|Default|GetselectedTile)
    (:Is%20Valid
      (Default|EventDeselectTile (Variables|Default|GetselectedTile)))
    (:Is%20Not%20Valid
      _))
  (Variables|Default|SetselectedTile selectedTile)
  (Default|EventNewPathAvailable (Variables|Default|GetPlayerController) (Variables|Default|GetPath)))

(event Custom|Event_NewTileOvered
  (params (Overed%20Tile :type BP%20Grid%20Tile%20Object%20Reference))
  (bind _selectedtile (Variables|Default|GetselectedTile))
  (Utilities|IsValid (Variables|Default|GetOveredTile)
    (:Is%20Valid
      (Default|EventEndOverTile (Variables|Default|GetOveredTile)))
    (:Is%20Not%20Valid
      _))
  (Variables|Default|SetOveredTile Overed%20Tile)
  (CallFunction|HighlightCurrentPath false)
  (if (and (Utilities|IsValid _selectedtile) (Utilities|IsValid (Variables|Default|GetOveredTile)))
    (CallFunction|FindPathtoTarget (Variables|/Game/BP_GridTile.BP_GridTile_C|GetgridIndex _selectedtile) (Variables|/Game/BP_GridTile.BP_GridTile_C|GetgridIndex (Variables|Default|GetOveredTile)))
    (CallFunction|HighlightCurrentPath true)))

(event EventBeginPlay
  (Rendering|Debug|FlushPersistentDebugLines)
  (Variables|Default|SetGridLocation (Transformation|GetWorldLocation (Variables|Default|GetDefaultSceneRoot)))
  (CallFunction|GenerateMapDatafromWorld)
  (CallFunction|SpawnTiles true)
  (Variables|Default|SetPlayerController (.AsBP%20Player%20Controller (Utilities|Casting|CastToBP_PlayerController (Game|GetPlayerController 0)))))

(event Collision|EventActorBeginOverlap
  (params (OtherActor :type Actor%20Object%20Reference)))

(event EventTick
  (params (DeltaSeconds :type Float%20%28single-precision%29)))

(fn ConstructionScript
  (bind _gridsizeworld (Variables|Default|GetGridSizeWorld))
  (Rendering|Debug|FlushPersistentDebugLines)
  (Variables|Default|SetGridLocation (Transformation|GetWorldLocation (Variables|Default|GetDefaultSceneRoot)))
  (Rendering|Debug|DrawDebugBox (Variables|Default|GetGridLocation) (Math|Vector|MakeVector (.y _gridsizeworld) (.x _gridsizeworld) 5.0) (Variables|Default|GetGridBoxColor) "0, 0, 0" 1e+05 1e+01)
  (Rendering|Debug|DrawDebugBox (CallFunction|GridBottomLeft) (Math|Vector|MakeVector 2e+01 2e+01 2e+01) (Variables|Default|GetBottomLeftColor) "0, 0, 0" 1e+05 1e+01)
  (CallFunction|GenerateMapDatafromWorld)
  (CallFunction|DrawTile))

(fn GridBottomLeft
  (return (- (- (Variables|Default|GetGridLocation) (* (Math|Vector|GetRightVector (Variables|Default|GetDefaultSceneRoot)) (.x (Variables|Default|GetGridSizeWorld)))) (* (Math|Vector|GetForwardVector (Variables|Default|GetDefaultSceneRoot)) (.y (Variables|Default|GetGridSizeWorld))))))

(fn GridTileNumber
  (bind _gridsizeworld (Variables|Default|GetGridSizeWorld))
  (bind _tilesize (Variables|Default|GetTileSize))
  (bind _returnvalue (/ _gridsizeworld _tilesize))
  (return (- (Math|Float|Round (.x _returnvalue)) 1) (- (Math|Float|Round (.y _returnvalue)) 1)))

(fn DrawTile
  (bind _keys (Utilities|Map|Keys (Variables|Default|Getstruct_Tiles)))
  (for _array_element _keys
    (CallFunction|MyDrawDebugPlane (.worldlocation (.Value (Utilities|Map|Find (Variables|Default|Getstruct_Tiles) _array_element))) (.groundtype (.Value (Utilities|Map|Find (Variables|Default|Getstruct_Tiles) _array_element))))))

(fn MySphereTrace
  (params (Location :type Vector) (TraceChannel :type ETraceTypeQuery%20Enum :default "TraceTypeQuery1"))
  (bind (_outhit _returnvalue) (Collision|SphereTraceByChannel Location Location (- (Variables|Default|GetTileSize) (Variables|Default|GetTileSizeMinus)) TraceChannel false 0 "None" true "(R=1.000000,G=0.000000,B=0.000000,A=1.000000)" "(R=0.000000,G=1.000000,B=0.000000,A=1.000000)" 2e+01))
  (return _returnvalue (.hitactor _outhit)))

(fn MyDrawDebugPlane
  (params (Location :type Vector) (GroundType :type Enum_GroundTypes%20Enum :default "NewEnumerator0"))
  (switch Utilities|FlowControl|Switch|SwitchonEnum_GroundTypes GroundType
    (:NewEnumerator0
      (LocalVariables|SetTitleColor "(R=1.000000,G=0.887153,B=0.887153,A=1.000000)"))
    (:NewEnumerator1
      (LocalVariables|SetTitleColor "(R=0.427327,G=0.546875,B=0.198490,A=1.000000)"))
    (:NewEnumerator2
      (LocalVariables|SetTitleColor "(R=0.939236,G=0.807359,B=0.073378,A=1.000000)"))
    (:NewEnumerator3
      (LocalVariables|SetTitleColor "(R=0.845486,G=0.000000,B=0.037123,A=1.000000)")))
  (Class|KismetSystemLibrary|DrawDebugPlane (Utilities|Struct|MakePlane (.Z (Math|Vector|BreakVector Location)) 0.0 0.0 1.0) Location (- (Variables|Default|GetTileSize) (Variables|Default|GetTileSizeMinus)) (LocalVariables|GetTitleColor) 1e+05))

(fn GenerateMapDatafromWorld
  (bind (_gridtilenumberx _gridtilenumbery) (CallFunction|GridTileNumber))
  (bind _tilesize (Variables|Default|GetTileSize))
  (bind _tilesize_2 (Variables|Default|GetTileSize))
  (for _index (range 0 _gridtilenumberx)
    (LocalVariables|SetX _index)
    (for _index_2 (range 0 _gridtilenumbery)
      (LocalVariables|SetY _index_2)
      (LocalVariables|SetTitlePosition (+ (CallFunction|GridBottomLeft) (* (Math|Vector|GetRightVector (Variables|Default|GetDefaultSceneRoot)) (+ (* (LocalVariables|GetX) (* _tilesize_2 2.0)) _tilesize_2)) (* (Math|Vector|GetForwardVector (Variables|Default|GetDefaultSceneRoot)) (+ (* (LocalVariables|GetY) (* _tilesize 2.0)) _tilesize))))
      (if (.ReturnValue (CallFunction|MySphereTrace (LocalVariables|GetTitlePosition) "TraceTypeQuery3"))
        (if (.ReturnValue (CallFunction|MySphereTrace (LocalVariables|GetTitlePosition) "TraceTypeQuery4"))
          (Utilities|Map|Add (Variables|Default|Getstruct_Tiles) (Math|Vector2D|MakeVector2D (Math|Conversions|ToFloat(Integer) (LocalVariables|GetX)) (Math|Conversions|ToFloat(Integer) (LocalVariables|GetY))) (Utilities|Struct|MakeStruct_Tiles 0 (Variables|/Game/BP_Base_Obstacle.BP_Base_Obstacle_C|GetEnum_GroundTypes (.AsBP%20Base%20Obstacle (Utilities|Casting|CastToBP_Base_Obstacle (.Actor (CallFunction|MySphereTrace (LocalVariables|GetTitlePosition) "TraceTypeQuery4"))))) (LocalVariables|GetTitlePosition) (Math|Vector2D|MakeVector2D (Math|Conversions|ToFloat(Integer) (LocalVariables|GetX)) (Math|Conversions|ToFloat(Integer) (LocalVariables|GetY))) 0 0 0 (CallFunction|GetTileCost (Variables|/Game/BP_Base_Obstacle.BP_Base_Obstacle_C|GetEnum_GroundTypes (.AsBP%20Base%20Obstacle (Utilities|Casting|CastToBP_Base_Obstacle (.Actor (CallFunction|MySphereTrace (LocalVariables|GetTitlePosition) "TraceTypeQuery4")))))) "(X=0.000000,Y=0.000000)"))
          (else
            (Utilities|Map|Add (Variables|Default|Getstruct_Tiles) (Math|Vector2D|MakeVector2D (Math|Conversions|ToFloat(Integer) (LocalVariables|GetX)) (Math|Conversions|ToFloat(Integer) (LocalVariables|GetY))) (Utilities|Struct|MakeStruct_Tiles 0 "NewEnumerator0" (LocalVariables|GetTitlePosition) (Math|Vector2D|MakeVector2D (Math|Conversions|ToFloat(Integer) (LocalVariables|GetX)) (Math|Conversions|ToFloat(Integer) (LocalVariables|GetY))) 0 0 0 (CallFunction|GetTileCost "NewEnumerator0") "(X=0.000000,Y=0.000000)"))))
        (else
          (Utilities|Map|Add (Variables|Default|Getstruct_Tiles) (Math|Vector2D|MakeVector2D (Math|Conversions|ToFloat(Integer) (LocalVariables|GetX)) (Math|Conversions|ToFloat(Integer) (LocalVariables|GetY))) (Utilities|Struct|MakeStruct_Tiles 0 "NewEnumerator4" (LocalVariables|GetTitlePosition) (Math|Vector2D|MakeVector2D (Math|Conversions|ToFloat(Integer) (LocalVariables|GetX)) (Math|Conversions|ToFloat(Integer) (LocalVariables|GetY))) 0 0 0 (CallFunction|GetTileCost "NewEnumerator4") "(X=0.000000,Y=0.000000)")))))))

(fn SpawnTiles
  (params (bSpawnNoneTile :type Boolean))
  (bind _struct_tiles (Variables|Default|Getstruct_Tiles))
  (bind _keys (Utilities|Map|Keys (Variables|Default|Getstruct_Tiles)))
  (for _array_element _keys
    (if (or bSpawnNoneTile (Utilities|Enum|NotEqual(Enum) (.groundtype (.Value (Utilities|Map|Find _struct_tiles _array_element))) "NewEnumerator4"))
      (bind _returnvalue (Game|SpawnActorfromClass "/Game/BP_GridTile.BP_GridTile_C" (Math|Conversions|ToTransform(Vector) (.worldlocation (.Value (Utilities|Map|Find _struct_tiles _array_element)))) "Undefined" 0 0))
      (Variables|/Game/BP_GridTile.BP_GridTile_C|SetgridIndex _returnvalue _array_element)
      (Variables|/Game/BP_GridTile.BP_GridTile_C|SetBP_Grid _returnvalue self)
      (Utilities|Map|Add _struct_tiles _array_element (Utilities|Struct|MakeStruct_Tiles _returnvalue (.groundtype (.Value (Utilities|Map|Find _struct_tiles _array_element))) (.worldlocation (.Value (Utilities|Map|Find _struct_tiles _array_element))) (.gridindex (.Value (Utilities|Map|Find _struct_tiles _array_element))) (.finalcost (.Value (Utilities|Map|Find _struct_tiles _array_element))) (.costfromstart (.Value (Utilities|Map|Find _struct_tiles _array_element))) (.estimatedcosttotarget (.Value (Utilities|Map|Find _struct_tiles _array_element))) (.tilecost (.Value (Utilities|Map|Find _struct_tiles _array_element))) (.previoustile (.Value (Utilities|Map|Find _struct_tiles _array_element))))))))

(fn GetTileCost
  (params (GroundTypes :type Enum_GroundTypes%20Enum :default "NewEnumerator0"))
  (switch Utilities|FlowControl|Switch|SwitchonEnum_GroundTypes GroundTypes
    (:NewEnumerator0
      (LocalVariables|SetCost 1))
    (:NewEnumerator1
      (LocalVariables|SetCost 2))
    (:NewEnumerator2
      (LocalVariables|SetCost 5))
    (:NewEnumerator3
      (LocalVariables|SetCost 999 :!label _label))
    (:NewEnumerator4
      (goto _label)))
  (return (LocalVariables|GetCost)))

(fn GetTileNeighbours
  (params (GridIndex :type Vector%202D%20Structure))
  (bind _output_get (LocalVariables|SetpossibleNeighbours (Utilities|Array|MakeArray "(X=1.000000,Y=0.000000)" "(X=0.000000,Y=1.000000)" "(X=-1.000000,Y=0.000000)" "(X=0.000000,Y=-1.000000)")))
  (for _array_element _output_get
    (if (.ReturnValue (Utilities|Map|Find (Variables|Default|Getstruct_Tiles) (+ _array_element GridIndex)))
      (if (and (Utilities|Enum|NotEqual(Enum) (.groundtype (.Value (Utilities|Map|Find (Variables|Default|Getstruct_Tiles) (+ _array_element GridIndex)))) "NewEnumerator4") (Utilities|Enum|NotEqual(Enum) (.groundtype (.Value (Utilities|Map|Find (Variables|Default|Getstruct_Tiles) (+ _array_element GridIndex)))) "NewEnumerator3"))
        (Utilities|Array|AddUnique (LocalVariables|GetoutNeighbours) (+ _array_element GridIndex)))))
  (return (LocalVariables|GetoutNeighbours)))

(fn GetEstimatedCosttoTarget
  (params (currentTile :type Vector%202D%20Structure) (TargetTile :type Vector%202D%20Structure))
  (bind _returnvalue (- currentTile TargetTile))
  (return (Math|Float|Round (+ (Math|Float|Absolute(Float) (.x _returnvalue)) (Math|Float|Absolute(Float) (.y _returnvalue))))))

(fn FindPathtoTarget
  (params (StartTile :type Vector%202D%20Structure) (TargetTile :type Vector%202D%20Structure))
  (bind _struct_tiles (Variables|Default|Getstruct_Tiles))
  (bind _struct_tiles_2 (Variables|Default|Getstruct_Tiles))
  (bind _struct_tiles_3 (Variables|Default|Getstruct_Tiles))
  (bind _struct_tiles_4 (Variables|Default|Getstruct_Tiles))
  (LocalVariables|SetStartTileL StartTile)
  (LocalVariables|SetTargetTileL TargetTile)
  (if (Math|Boolean|ANDBoolean (Utilities|Enum|NotEqual(Enum) (.groundtype (.Value (Utilities|Map|Find (Variables|Default|Getstruct_Tiles) (LocalVariables|GetTargetTileL)))) "NewEnumerator4") (Utilities|Enum|NotEqual(Enum) (.groundtype (.Value (Utilities|Map|Find (Variables|Default|Getstruct_Tiles) (LocalVariables|GetTargetTileL)))) "NewEnumerator3") (.ReturnValue (Utilities|Map|Find (Variables|Default|Getstruct_Tiles) (LocalVariables|GetTargetTileL))))
    (Utilities|FlowControl|Sequence
      (:then_0
        (bind _keys (Utilities|Map|Keys (Variables|Default|Getstruct_Tiles)))
        (for _array_element _keys
          (Utilities|Map|Add _struct_tiles_3 _array_element (Utilities|Struct|MakeStruct_Tiles (.tileactor (.Value (Utilities|Map|Find _struct_tiles_3 _array_element))) (.groundtype (.Value (Utilities|Map|Find _struct_tiles_3 _array_element))) (.worldlocation (.Value (Utilities|Map|Find _struct_tiles_3 _array_element))) (.gridindex (.Value (Utilities|Map|Find _struct_tiles_3 _array_element))) 999 999 999 (.tilecost (.Value (Utilities|Map|Find _struct_tiles_3 _array_element))) "(X=0.000000,Y=0.000000)")))
        (Utilities|Map|Add _struct_tiles (LocalVariables|GetStartTileL) (Utilities|Struct|MakeStruct_Tiles (.tileactor (.Value (Utilities|Map|Find _struct_tiles (LocalVariables|GetStartTileL)))) (.groundtype (.Value (Utilities|Map|Find _struct_tiles (LocalVariables|GetStartTileL)))) (.worldlocation (.Value (Utilities|Map|Find _struct_tiles (LocalVariables|GetStartTileL)))) (.gridindex (.Value (Utilities|Map|Find _struct_tiles (LocalVariables|GetStartTileL)))) (CallFunction|GetEstimatedCosttoTarget (LocalVariables|GetStartTileL) (LocalVariables|GetTargetTileL)) 0 (CallFunction|GetEstimatedCosttoTarget (LocalVariables|GetStartTileL) (LocalVariables|GetTargetTileL)) (.tilecost (.Value (Utilities|Map|Find _struct_tiles (LocalVariables|GetStartTileL)))) "(X=0.000000,Y=0.000000)")))
      (:then_1
        (bind _output_get (LocalVariables|SetCurrentTile (LocalVariables|GetStartTileL)))
        (Utilities|Array|AddUnique (LocalVariables|GetopenSet) _output_get)
        (while (> (Utilities|Array|Length (LocalVariables|GetopenSet)) 0)
          (LocalVariables|SetopenSetCheapest (Utilities|Array|Get(acopy) (LocalVariables|GetopenSet)))
          (for _array_element_2 (LocalVariables|GetopenSet)
            (if (< (.finalcost (.Value (Utilities|Map|Find _struct_tiles_2 _array_element_2))) (.finalcost (.Value (Utilities|Map|Find _struct_tiles_2 (LocalVariables|GetopenSetCheapest)))))
              (LocalVariables|SetopenSetCheapest _array_element_2 :!label _label)
              (elif (== (.finalcost (.Value (Utilities|Map|Find _struct_tiles_2 _array_element_2))) (.finalcost (.Value (Utilities|Map|Find _struct_tiles_2 (LocalVariables|GetopenSetCheapest)))))
                (if (< (.estimatedcosttotarget (.Value (Utilities|Map|Find _struct_tiles_2 _array_element_2))) (.estimatedcosttotarget (.Value (Utilities|Map|Find _struct_tiles_2 (LocalVariables|GetopenSetCheapest)))))
                  (goto _label)))))
          (LocalVariables|SetCurrentTile (LocalVariables|GetopenSetCheapest))
          (Utilities|Array|RemoveItem (LocalVariables|GetopenSet) (LocalVariables|GetCurrentTile))
          (Utilities|Array|AddUnique (LocalVariables|GetclosedSet) (LocalVariables|GetCurrentTile))
          (for _array_element_3 (CallFunction|GetTileNeighbours (LocalVariables|GetCurrentTile))
            (LocalVariables|SetCurrentNeighbour _array_element_3)
            (if (not (Utilities|Array|ContainsItem (LocalVariables|GetclosedSet) (LocalVariables|GetCurrentNeighbour)))
              (LocalVariables|SetcurrentNeighbourCostFromStart (+ (.costfromstart (.Value (Utilities|Map|Find (Variables|Default|Getstruct_Tiles) (LocalVariables|GetCurrentTile)))) (.tilecost (.Value (Utilities|Map|Find (Variables|Default|Getstruct_Tiles) (LocalVariables|GetCurrentNeighbour))))))
              (if (not (Utilities|Array|ContainsItem (LocalVariables|GetopenSet) (LocalVariables|GetCurrentNeighbour)))
                (Utilities|Array|AddUnique (LocalVariables|GetopenSet) (LocalVariables|GetCurrentNeighbour))
                (Utilities|Map|Add _struct_tiles_4 (LocalVariables|GetCurrentNeighbour) (Utilities|Struct|MakeStruct_Tiles (.tileactor (.Value (Utilities|Map|Find _struct_tiles_4 (LocalVariables|GetCurrentNeighbour)))) (.groundtype (.Value (Utilities|Map|Find _struct_tiles_4 (LocalVariables|GetCurrentNeighbour)))) (.worldlocation (.Value (Utilities|Map|Find _struct_tiles_4 (LocalVariables|GetCurrentNeighbour)))) (.gridindex (.Value (Utilities|Map|Find _struct_tiles_4 (LocalVariables|GetCurrentNeighbour)))) (+ (LocalVariables|GetcurrentNeighbourCostFromStart) (CallFunction|GetEstimatedCosttoTarget (LocalVariables|GetCurrentNeighbour) (LocalVariables|GetTargetTileL))) (LocalVariables|GetcurrentNeighbourCostFromStart) (CallFunction|GetEstimatedCosttoTarget (LocalVariables|GetCurrentNeighbour) (LocalVariables|GetTargetTileL)) (.tilecost (.Value (Utilities|Map|Find _struct_tiles_4 (LocalVariables|GetCurrentNeighbour)))) (LocalVariables|GetCurrentTile)) :!label _label_2)
                (if (Math|Vector|Equal(Vector) (LocalVariables|GetCurrentNeighbour) (LocalVariables|GetTargetTileL) 0.0001)
                  (Variables|Default|SetPath (CallFunction|RetracePath (LocalVariables|GetTargetTileL) (LocalVariables|GetStartTileL)))
                  (return))
                (elif (< (LocalVariables|GetcurrentNeighbourCostFromStart) (.costfromstart (.Value (Utilities|Map|Find _struct_tiles_4 (LocalVariables|GetCurrentNeighbour)))))
                  (goto _label_2))))))
        (return)))))

(fn RetracePath
  (params (TargetTile :type Vector%202D%20Structure) (StartTile :type Vector%202D%20Structure))
  (LocalVariables|SetcurrentTile TargetTile)
  (while (Math|Vector|NotEqual(Vector) (LocalVariables|GetcurrentTile) StartTile 0.0001)
    (Utilities|Array|AddUnique (LocalVariables|GetreversedPath) (LocalVariables|GetcurrentTile))
    (LocalVariables|SetcurrentTile (.previoustile (.Value (Utilities|Map|Find (Variables|Default|Getstruct_Tiles) (LocalVariables|GetcurrentTile))))))
  (bind _arrayelement (Utilities|Array|ReverseforEachLoop (LocalVariables|GetreversedPath))
    (:LoopBody
      (Utilities|Array|AddUnique (LocalVariables|GetOutPath) _arrayelement))
    (:Completed
      (return (LocalVariables|GetOutPath)))))

(fn HighlightCurrentPath
  (params (isforHighlight :type Boolean))
  (for _array_element (Variables|Default|GetPath)
    (Utilities|IsValid (.tileactor (.Value (Utilities|Map|Find (Variables|Default|Getstruct_Tiles) _array_element)))
      (:Is%20Valid
        (Default|EventIsinPath (.tileactor (.Value (Utilities|Map|Find (Variables|Default|Getstruct_Tiles) _array_element))) isforHighlight)))))